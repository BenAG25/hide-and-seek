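; BP_HS_PlayerController is the player controller for the Hide and Seek mode.
; On BeginPlay it registers the default and mouse-look Enhanced Input mapping contexts, only for the local controller.
; A debug key on F casts player state 0 to BP_HS_PlayerState and calls its role-printing debug function.
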(event EventBeginPlay
  (Utilities|FlowControl|Sequence
    (:then_0
      (CallFunction|InputSystem))))

(event Input|KeyboardEvents|DebugKeyF
  (params (Key :type Key%20Structure :default "None") (ActionValue :type Input%20Action%20Value%20Structure))
  (:Pressed
    (bind _asbp_hs_player_state (Utilities|Casting|CastToBP_HS_PlayerState (Game|GetPlayerState 0)))
    (Default|DebugPrintRoles _asbp_hs_player_state)))

(fn ConstructionScript)

(fn InputSystem
  (bind _returnvalue (PlayerController|LocalPlayerSubsystems|GetEnhancedInputLocalPlayerSubsystem))
  (if (Pawn|IsLocalController)
    (Input|AddMappingContext _returnvalue "/Game/Input/IMC_MouseLook.IMC_MouseLook" 0 "(bIgnoreAllPressedKeysUntilRelease=True,bForceImmediately=False,bNotifyUserSettings=False)")
    (Input|AddMappingContext _returnvalue "/Game/Input/IMC_Default.IMC_Default" 0 "(bIgnoreAllPressedKeysUntilRelease=True,bForceImmediately=False,bNotifyUserSettings=False)")))