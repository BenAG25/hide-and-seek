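; Game mode for a Hide and Seek game that hands out player roles once enough players have joined.
; Each login calls StartMatch, which runs AssingRoles when the PlayerArray count reaches MaxPlayers.
; AssingRoles gives one role at index 0 and another at later indices, but always writes to player state 0 instead of the looped element.
; A Shuffle node is present but never runs.
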(event `self.K2_PostLogin`
  (params (NewPlayer :type "PlayerController Object Reference"))
  (`self.StartMatch`))

(event `StartMatch`
  (if (>= (`KismetArrayLibrary.Array_Length` (`GameStateBase.PlayerArray` (`GameplayStatics.GetGameState`))) (`self.MaxPlayers`))
    (`self.AssingRoles`)))

(fn `AssingRoles`
  (for (_ _array_index) (`GameStateBase.PlayerArray` (`GameplayStatics.GetGameState`))
    (bind _asbp_hs_player_state (cast `/Game/_HideAndSeek/Core/BP_HS_PlayerState` (`GameplayStatics.GetPlayerState` 0)))
    (if (== _array_index 0)
      (set `/Game/_HideAndSeek/Core/BP_HS_PlayerState.PlayerRole` "NewEnumerator1" _asbp_hs_player_state)
      (else
        (set `/Game/_HideAndSeek/Core/BP_HS_PlayerState.PlayerRole` "NewEnumerator2" _asbp_hs_player_state)))))

(fn `UserConstructionScript`)