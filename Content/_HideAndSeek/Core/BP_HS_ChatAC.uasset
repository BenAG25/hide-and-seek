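; Actor component on the Hide and Seek player controller that provides in-game text chat between players.
; On BeginPlay it creates the chat UI for the local controller and caches its chat box, which Enter focuses and the mouse wheel scrolls.
; A server event relays each message through every player's controller to that player's chat component, whose owning-client event adds it to the chat box.
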(event `self.ReceiveBeginPlay`
  (if (`Controller.IsLocalPlayerController` (cast `/Game/_HideAndSeek/Core/BP_HS_PlayerController` (`self.GetOwner`) :!pure true))
    (bind _returnvalue (`|CreateWidget` "/Game/_HideAndSeek/UI/WBP_ChatUI.WBP_ChatUI_C"))
    (bind _output_get (set `self.Chat_UI_Ref` _returnvalue))
    (`UserWidget.AddToViewport` _output_get 0)
    (set `self.ChatBox_Ref` (`/Game/_HideAndSeek/UI/WBP_ChatUI.WBP_ChatBox` _output_get))))

(event `Key|Enter`
  (params (Key :type "Key Structure"))
  (:`Pressed`
    (`/Game/_HideAndSeek/UI/WBP_ChatBox.FocusChat` (`self.ChatBox_Ref`))))

(event `Key|MouseScrollUp`
  (params (Key :type "Key Structure"))
  (:`Pressed`
    (`/Game/_HideAndSeek/UI/WBP_ChatBox.Scroll` (`self.ChatBox_Ref`) true)))

(event `Key|MouseScrollDown`
  (params (Key :type "Key Structure"))
  (:`Pressed`
    (`/Game/_HideAndSeek/UI/WBP_ChatBox.Scroll` (`self.ChatBox_Ref`) false)))

(event `SendChatMessage_OnServer`
  (params (Message :type String))
  (for _array_element (`GameStateBase.PlayerArray` (`GameplayStatics.GetGameState`))
    (`self.AddChatMessageOnOwningClient` (`Actor.K2_GetComponentsByClass` (`PlayerState.GetPlayerController` _array_element) "BP_HS_ChatAC_C") Message)))

(event `AddChatMessageOnOwningClient`
  (params (Message :type String))
  (`/Game/_HideAndSeek/UI/WBP_ChatBox.AddChatMessage` (`self.ChatBox_Ref`) Message))