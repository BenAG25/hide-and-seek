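; BP_HS_GameState is the Hide and Seek game state, which delivers chat messages to players' screens.
; A multicast event takes a sender name and message, then gets the local BP_HS_PlayerController through player index 0.
; It creates a WBP_ChatMessage formatted as "sender: message", appends it to that controller's chat scroll box, scrolls to the end and briefly shows the chat.
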(event `Multicast_BroadcastChatMessage`
  (params (SenderName :type String) (Message :type String))
  (bind _asbp_hs_player_controller (cast `/Game/_HideAndSeek/Core/BP_HS_PlayerController` (`GameplayStatics.GetPlayerController` 0)))
  (bind _returnvalue (`|CreateWidget` "/Game/_HideAndSeek/UI/WBP_ChatMessage.WBP_ChatMessage_C" _asbp_hs_player_controller (`|FormatText` "{SenderName}: {Message}" (`KismetTextLibrary.Conv_StringToText` SenderName) (`KismetTextLibrary.Conv_StringToText` Message))))
  (bind _chatwidget (`/Game/_HideAndSeek/Core/BP_HS_PlayerController.ChatWidget` _asbp_hs_player_controller))
  (bind _chatscrollbox (`/Game/_HideAndSeek/UI/WBP_ChatMessage.ChatScrollBox` _chatwidget))
  (`PanelWidget.AddChild` _chatscrollbox _returnvalue)
  (`ScrollBox.ScrollToEnd` _chatscrollbox)
  (`/Game/_HideAndSeek/UI/WBP_ChatMessage.ShowChatTemporarily` _chatwidget))

(fn `UserConstructionScript`)